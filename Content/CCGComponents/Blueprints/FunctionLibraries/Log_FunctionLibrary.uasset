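; Blueprint function library for the card game's in-game message log.
; AddMessageToLog sends a message and color to the calling player's game UI MessageManager, after validity checks on both the UI reference and the manager.
; Companion functions use FormatText to build ability log strings for card cloning, card pickup and attack gains from a card name or amount, returning them rather than logging them.
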(fn `AddMessageToLog`
  (params (CallingPlayer :type "/Game/CCGComponents/Blueprints/CardGamePlayerController Object Reference") (Message :type String) (`Specified Color` :type "LinearColor Structure"))
  (bind _playergameui_ref (`/Game/CCGComponents/Blueprints/CardGamePlayerController.PlayerGameUI_Ref` CallingPlayer))
  (bind _message_manager (`/Game/CCGComponents/Blueprints/Widgets/Gameplay/PlayerGameUI.Message_Manager` _playergameui_ref))
  (`/Engine/EditorBlueprintResources/StandardMacros.IsValid` _playergameui_ref
    (:`Is Valid`
      (`/Engine/EditorBlueprintResources/StandardMacros.IsValid` _message_manager
        (:`Is Valid`
          (`/Game/CCGComponents/Blueprints/Widgets/Additional/Message_Manager.LogMessage` _message_manager CallingPlayer Message `Specified Color`))
        (:`Is Not Valid`
          _)))
    (:`Is Not Valid`
      _))
  (return))

(fn `CloneCard_LogMessage`
  (params (CardName :type Text) (AbilityInt :type Integer))
  (returns (ReturnString :type String))
  (return (`KismetTextLibrary.Conv_TextToString` (`|FormatText` "{cardname} cloned up to + {AbilityInt} times!" CardName (`KismetTextLibrary.Conv_IntToText` AbilityInt)))))

(fn `IncreaseAttack_LogMessage`
  (params (CardName :type Text) (AbilityInt :type Integer))
  (returns (ReturnString :type String))
  (return (`KismetTextLibrary.Conv_TextToString` (`|FormatText` "{cardname} gained + {AbilityInt} Attack" CardName (`KismetTextLibrary.Conv_IntToText` AbilityInt)))))

(fn `PickupCard(s)_LogMessage`
  (params (AbilityInt :type Integer))
  (returns (ReturnString :type String))
  (return (`KismetTextLibrary.Conv_TextToString` (`|FormatText` "Player picked up + {AbilityInt} cards" (`KismetTextLibrary.Conv_IntToText` AbilityInt)))))