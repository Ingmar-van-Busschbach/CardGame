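; Function library that resolves card attacks on other cards and players in the card game.
; Non-simple attacks validate both sides, spend a turn point and multicast the attack; SimpleDamage skips all three.
; Damage uses the attacker's Attack unless overridden, then is recorded in the GameState's battle history.
; Validation checks turn points, attack, health, graveyard state and target permissions, plus data-driven interaction conditions that report the first failed rule.
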(fn `ChargeInteractionPoints`
  (params (CardToCharge :type "/Game/CCGComponents/Blueprints/Gameplay/3DCard Object Reference") (Cost :type Integer))
  (returns (Success :type Boolean))
  (bind _turnpoints (`/Game/CCGComponents/Blueprints/Gameplay/3DCard.TurnPoints` CardToCharge))
  (if (>= _turnpoints 1)
    (set `/Game/CCGComponents/Blueprints/Gameplay/3DCard.TurnPoints` (- _turnpoints Cost) CardToCharge)
    (return true)
    (else
      (return false))))

(fn `Deal Damage to Card`
  (params (SimpleDamage :type Boolean :default false) (TalkingCard :type "/Game/CCGComponents/Blueprints/Gameplay/3DCard Object Reference") (RecievingCard :type "/Game/CCGComponents/Blueprints/Gameplay/3DCard Object Reference") (DamageOverride :type Integer))
  (returns (Success :type Boolean) (CallingCardCondition :type "/Game/CCGComponents/Blueprints/Enums/Gameplay_Enums/InteractionConditions_Enum Enum") (TalkingCardCondition :type "/Game/CCGComponents/Blueprints/Enums/Gameplay_Enums/InteractionConditions_Enum Enum"))
  (locals (InteractionTalkingCard :type "/Game/CCGComponents/Blueprints/Gameplay/3DCard Object Reference") (InteracitionRecievingCard :type "/Game/CCGComponents/Blueprints/Gameplay/3DCard Object Reference") (CallingCardConditionFailure :type "/Game/CCGComponents/Blueprints/Enums/Gameplay_Enums/InteractionConditions_Enum Enum") (TalkingCardConditionFailure :type "/Game/CCGComponents/Blueprints/Enums/Gameplay_Enums/InteractionConditions_Enum Enum"))
  (bind _interactiontalkingcard (`local.InteractionTalkingCard`))
  (bind (_returnvalue _callingcardconditionfailure _talkingcardconditionfailure) (`self.ValidateCardInteraction` (`local.InteractionTalkingCard`) (`local.InteracitionRecievingCard`)))
  (set `local.InteractionTalkingCard` TalkingCard)
  (set `local.InteracitionRecievingCard` RecievingCard)
  (if SimpleDamage
    ;[1 0.4639 0.1607 0.3] Attack Recieving Cards health
    (message `/Game/CCGComponents/Blueprints/Interface/CardInteraction_Interface.TakesDamage` (`local.InteracitionRecievingCard`) (`local.InteractionTalkingCard`) 0 (select `bool` (> DamageOverride 0) :`false` (`.Attack` (`/Game/CCGComponents/Blueprints/FunctionLibraries/Misc_FunctionLibrary.ReadInteractingCardData` (`local.InteractionTalkingCard`))) :`true` DamageOverride) :!label _label)
    ;[0.4374 0.9901 1 0.3] Record Battle History Result
    (bind _ascard_game_state (cast `/Game/CCGComponents/Blueprints/CardGameState` (`GameplayStatics.GetGameState` null))
      (:`then`
        _)
      (:`CastFailed`
        (return false (`local.CallingCardConditionFailure`) (`local.TalkingCardConditionFailure`))))
    (else
      (if _returnvalue
        (bind _success (`self.ChargeInteractionPoints` (`local.InteractionTalkingCard`) 1))
        (if _success
          (`/Game/CCGComponents/Blueprints/Gameplay/3DCard.Multicast_Attacking` (`local.InteractionTalkingCard`) (`local.InteracitionRecievingCard`))
          (goto _label)
          (else
            _))
        (else
          (set `local.CallingCardConditionFailure` _callingcardconditionfailure)
          (set `local.TalkingCardConditionFailure` _talkingcardconditionfailure)))
      (return false (`local.CallingCardConditionFailure`) (`local.TalkingCardConditionFailure`))))
  (`/Game/CCGComponents/Blueprints/CardGameState.RecordBattleHistory` _ascard_game_state (make `/Game/CCGComponents/CardGame/Structs/GameStructs/BattleHistory_Struct` (`/Game/CCGComponents/Blueprints/Gameplay/3DCard.OwningPlayerID` _interactiontalkingcard) "NewEnumerator1" (`/Game/CCGComponents/Blueprints/Gameplay/3DCard.CardDataStruct` _interactiontalkingcard) (`/Game/CCGComponents/Blueprints/Gameplay/3DCard.CardDataStruct` (`local.InteracitionRecievingCard`))))
  (return true (`local.CallingCardConditionFailure`) (`local.TalkingCardConditionFailure`)))

(fn `Deal Damage to Player`
  (params (SimpleDamage :type Boolean :default false) (TalkingCard :type "/Game/CCGComponents/Blueprints/Gameplay/3DCard Object Reference") (BoardPlayer :type "/Game/CCGComponents/Blueprints/Gameplay/BoardPlayer Object Reference") (DamageOverride :type Integer))
  (returns (Success :type Boolean) (InteractionConditionFailure :type "/Game/CCGComponents/Blueprints/Enums/Gameplay_Enums/InteractionConditions_Enum Enum"))
  (locals (InteractionTalkingCard :type "/Game/CCGComponents/Blueprints/Gameplay/3DCard Object Reference") (InteractionRecievingPlayer :type "/Game/CCGComponents/Blueprints/Gameplay/BoardPlayer Object Reference") (ConditionFailure :type "/Game/CCGComponents/Blueprints/Enums/Gameplay_Enums/InteractionConditions_Enum Enum"))
  (bind _interactiontalkingcard (`local.InteractionTalkingCard`))
  (bind (_returnvalue _conditionfailure) (`self.ValidatePlayerInteraction` (`local.InteractionTalkingCard`) (`local.InteractionRecievingPlayer`)))
  (set `local.InteractionTalkingCard` TalkingCard)
  (set `local.InteractionRecievingPlayer` BoardPlayer)
  (if SimpleDamage
    ;[1 0.1804 0.1804 0.298] Attack Enemy Player's Health
    (message `/Game/CCGComponents/Blueprints/Interface/PlayerState_Interface.DecreasePlayerHealth` (`/Game/CCGComponents/Blueprints/FunctionLibraries/Controller_FunctionLibrary.GetControllerPlayerState(ServerOnly)` (`/Game/CCGComponents/Blueprints/Gameplay/BoardPlayer.PlayerIndex` (`local.InteractionRecievingPlayer`))) (select `bool` (> DamageOverride 0) :`false` (`.Attack` (`/Game/CCGComponents/Blueprints/FunctionLibraries/Misc_FunctionLibrary.ReadInteractingCardData` (`local.InteractionTalkingCard`))) :`true` DamageOverride) :!label _label)
    ;[0.4374 0.9901 1 0.3] Record Battle History Result
    (bind _ascard_game_state (cast `/Game/CCGComponents/Blueprints/CardGameState` (`GameplayStatics.GetGameState` null))
      (:`then`
        _)
      (:`CastFailed`
        (return false (`local.ConditionFailure`))))
    (else
      (if _returnvalue
        (bind _success (`self.ChargeInteractionPoints` (`local.InteractionTalkingCard`) 1))
        (if _success
          (`/Game/CCGComponents/Blueprints/Gameplay/3DCard.Multicast_Attacking` (`local.InteractionTalkingCard`) (`local.InteractionRecievingPlayer`))
          (goto _label)
          (else
            _))
        (else
          (set `local.ConditionFailure` _conditionfailure)))
      (return false (`local.ConditionFailure`))))
  (`/Game/CCGComponents/Blueprints/CardGameState.RecordBattleHistory` _ascard_game_state (make `/Game/CCGComponents/CardGame/Structs/GameStructs/BattleHistory_Struct` (`/Game/CCGComponents/Blueprints/Gameplay/3DCard.OwningPlayerID` _interactiontalkingcard) "NewEnumerator2" (`/Game/CCGComponents/Blueprints/Gameplay/3DCard.CardDataStruct` _interactiontalkingcard) (struct :`Name` "NSLOCTEXT(\"[9BF66B85476B4671586CAFB4B5341AF5]\", \"86C97B6F40E20C25EB24249DD5ED19D6\", \"[Name]\")" :`Class` "NewEnumerator0" :`Type` "NewEnumerator0" :`Rarity` "NewEnumerator0" :`Visual` (struct) :`Attack` (struct :`CanAttackPlayer` true :`CanAttackCards` true :`Damage_Type` "NewEnumerator0") :`Health` (struct :`Health` 1) :`Abilities` "(())" :`Description` (struct :`Description` "(Description Top)") :`Placement_Settings` (struct :`Owner` "NewEnumerator0" :`Mana_Cost` 1) :`DeckSettings` (struct :`Unlocked` true :`AddToPlayerDeck` true :`MaxNumInDeck` 3 :`ScreenSize` (512.0 768.0)) :`Card_System_Data` (struct)) (`/Game/CCGComponents/Blueprints/Gameplay/BoardPlayer.PlayerIndex` (`local.InteractionRecievingPlayer`))))
  (return true (`local.ConditionFailure`)))

(fn `IsSameOwningPlayer`
  (params (TalkingCard :type "/Game/CCGComponents/Blueprints/Gameplay/3DCard Object Reference") (RecievingCard :type "/Game/CCGComponents/Blueprints/Gameplay/3DCard Object Reference"))
  (returns (ReturnValue :type Boolean))
  (return (== (`/Game/CCGComponents/Blueprints/Gameplay/3DCard.OwningPlayerID` TalkingCard) (`/Game/CCGComponents/Blueprints/Gameplay/3DCard.OwningPlayerID` RecievingCard))))

(fn `ValidateCardInteraction`
  (params (TalkingCard :type "/Game/CCGComponents/Blueprints/Gameplay/3DCard Object Reference") (RecievingCard :type "/Game/CCGComponents/Blueprints/Gameplay/3DCard Object Reference"))
  (returns (ReturnValue :type Boolean) (CallingCardConditionFailure :type "/Game/CCGComponents/Blueprints/Enums/Gameplay_Enums/InteractionConditions_Enum Enum") (TalkingCardConditionFailure :type "/Game/CCGComponents/Blueprints/Enums/Gameplay_Enums/InteractionConditions_Enum Enum"))
  (bind (_returnvalid _conditionfailure) (`self.ValidateCardInteractionConditions` TalkingCard RecievingCard true))
  (bind (_returnvalid_2 _conditionfailure_2) (`self.ValidateCardInteractionConditions` TalkingCard RecievingCard))
  (return (and (and (> (`/Game/CCGComponents/Blueprints/Gameplay/3DCard.TurnPoints` TalkingCard) 0) (> (`/Game/CCGComponents/Blueprints/Gameplay/3DCard.Attack` TalkingCard) 0) (not (`/Game/CCGComponents/Blueprints/Gameplay/3DCard.bInGraveyard` TalkingCard)) (`.CanAttackCards_7_A4ED3D324F996F8266DA66A200150594` (break `/Game/CCGComponents/CardGame/Structs/CardStructs/Attack_Struct` (`.Attack_42_C92CE63C4661BD819996CEA4A1AA573F` (break `/Game/CCGComponents/CardGame/Structs/CardStructs/Card_Struct` (`/Game/CCGComponents/Blueprints/Gameplay/3DCard.CardDataStruct` TalkingCard)))))) (and (> (`/Game/CCGComponents/Blueprints/Gameplay/3DCard.Health` RecievingCard) 0) (not (`/Game/CCGComponents/Blueprints/Gameplay/3DCard.bInGraveyard` RecievingCard))) (and _returnvalid_2 _returnvalid)) _conditionfailure_2 _conditionfailure))

(fn `ValidateCardInteractionConditions`
  (params (TalkingCard :type "/Game/CCGComponents/Blueprints/Gameplay/3DCard Object Reference") (RecievingCard :type "/Game/CCGComponents/Blueprints/Gameplay/3DCard Object Reference") (RecievingCardConditions :type Boolean))
  (returns (ReturnValid :type Boolean) (ConditionFailure :type "/Game/CCGComponents/Blueprints/Enums/Gameplay_Enums/InteractionConditions_Enum Enum"))
  (locals (RecievingCard_Ref :type "/Game/CCGComponents/Blueprints/Gameplay/3DCard Object Reference") (TalkingCard_Ref :type "/Game/CCGComponents/Blueprints/Gameplay/3DCard Object Reference") (Valid :type Boolean) (InteractionCondition :type "/Game/CCGComponents/Blueprints/Enums/Gameplay_Enums/InteractionConditions_Enum Enum"))
  (bind _owningplayerid (`/Game/CCGComponents/Blueprints/Gameplay/3DCard.OwningPlayerID` (`local.TalkingCard_Ref`)))
  (set `local.TalkingCard_Ref` TalkingCard)
  (set `local.InteractionCondition` "NewEnumerator15")
  (`/Engine/EditorBlueprintResources/StandardMacros.IsValid` RecievingCard
    (:`Is Valid`
      (set `local.RecievingCard_Ref` RecievingCard))
    (:`Is Not Valid`
      _))
  (set `local.Valid` true)
  (for _array_element (select `bool` RecievingCardConditions :`false` (`.InteractionConditions_25_3638065048E26F7EEBC0419DB6B67BC8` (break `/Game/CCGComponents/CardGame/Structs/CardStructs/CardSystemData_Struct` (`.Card_System_Data_67_CD7BE5344ECD9A4915193697F6EA94B7` (break `/Game/CCGComponents/CardGame/Structs/CardStructs/Card_Struct` (`/Game/CCGComponents/Blueprints/Gameplay/3DCard.CardDataStruct` (`local.TalkingCard_Ref`)))))) :`true` (`.InteractionConditions_25_3638065048E26F7EEBC0419DB6B67BC8` (break `/Game/CCGComponents/CardGame/Structs/CardStructs/CardSystemData_Struct` (`.Card_System_Data_67_CD7BE5344ECD9A4915193697F6EA94B7` (break `/Game/CCGComponents/CardGame/Structs/CardStructs/Card_Struct` (`/Game/CCGComponents/Blueprints/Gameplay/3DCard.CardDataStruct` (`local.RecievingCard_Ref`)))))))
    (set `local.InteractionCondition` _array_element)
    ;[1 0.5998 0.226 0.3] Check Condition
    (switch `/Game/CCGComponents/Blueprints/Enums/Gameplay_Enums/InteractionConditions_Enum` _array_element
      (:`NewEnumerator9`
        (if (not (`/Game/CCGComponents/Blueprints/FunctionLibraries/CardConditions_FunctionLibrary.ConditionIfPlacedOnOwnedPlacement` _owningplayerid (`local.RecievingCard_Ref`)))
          (set `local.Valid` false :!label _label)
          (break)))
      (:`NewEnumerator10`
        (if (not (`/Game/CCGComponents/Blueprints/FunctionLibraries/CardConditions_FunctionLibrary.ConditionIfPlacedOnOwnedPlacement` _owningplayerid (`local.RecievingCard_Ref`) true))
          (goto _label)))
      (:`NewEnumerator0`
        (if (not (`/Game/CCGComponents/Blueprints/FunctionLibraries/CardConditions_FunctionLibrary.ConditionIfRecievingCardType` (`local.RecievingCard_Ref`) "NewEnumerator0"))
          (goto _label)))
      (:`NewEnumerator11`
        (if (not (`/Game/CCGComponents/Blueprints/FunctionLibraries/CardConditions_FunctionLibrary.ConditionIsNotOwningPlayer` _owningplayerid (`local.RecievingCard_Ref`)))
          (goto _label)))))
  (if (`local.Valid`)
    (set `local.InteractionCondition` "NewEnumerator15"))
  (return (`local.Valid`) (`local.InteractionCondition`)))

(fn `ValidatePlayerInteraction`
  (params (TalkingCard :type "/Game/CCGComponents/Blueprints/Gameplay/3DCard Object Reference") (RecievingBoardPlayer :type "/Game/CCGComponents/Blueprints/Gameplay/BoardPlayer Object Reference"))
  (returns (ReturnValue :type Boolean) (ConditionFailure :type "/Game/CCGComponents/Blueprints/Enums/Gameplay_Enums/InteractionConditions_Enum Enum"))
  (bind (_returnvalid _conditionfailure) (`self.ValidateCardInteractionConditions` TalkingCard))
  (return (and (and (> (`/Game/CCGComponents/Blueprints/Gameplay/3DCard.TurnPoints` TalkingCard) 0) (> (`/Game/CCGComponents/Blueprints/Gameplay/3DCard.Attack` TalkingCard) 0) (not (`/Game/CCGComponents/Blueprints/Gameplay/3DCard.bInGraveyard` TalkingCard)) (`.CanAttackPlayer_5_7DFF2313434E771DB380A5AE05B24EAF` (break `/Game/CCGComponents/CardGame/Structs/CardStructs/Attack_Struct` (`.Attack_42_C92CE63C4661BD819996CEA4A1AA573F` (break `/Game/CCGComponents/CardGame/Structs/CardStructs/Card_Struct` (`/Game/CCGComponents/Blueprints/Gameplay/3DCard.CardDataStruct` TalkingCard)))))) (> (`/Game/CCGComponents/Blueprints/FunctionLibraries/Controller_FunctionLibrary.GetControllersStateProfile(ServerOnly)` (`/Game/CCGComponents/Blueprints/Gameplay/BoardPlayer.PlayerIndex` RecievingBoardPlayer)) 0) _returnvalid) _conditionfailure))